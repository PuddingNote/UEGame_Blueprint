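; Player character Blueprint with Enhanced Input movement and look, weapon pickup, and a montage-based melee combo attack.
; Collected weapons snap to a mesh socket and enable attacking.
; Attacking from Peace enters Battle and plays the montage; further presses set NextCombo from the current section, and AttackEnd resets both.
; Attack-check begin and end events are forwarded to the held BP_Weapon.
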(event `self.ReceiveBeginPlay`
  ; 키보드 Move 입력
  (`EnhancedInputSubsystemInterface.AddMappingContext` (pcsubsystem `EnhancedInputLocalPlayerSubsystem` (`GameplayStatics.GetPlayerController` 0)) "/Game/Blueprints/Inputs/IMC_Character.IMC_Character" 0 (struct)))

(event `EnhancedInput|/Game/Blueprints/Inputs/Actions/IA_Move`
  (params (ActionValue :type "Vector2D Structure") (ElapsedSeconds :type "Float (double-precision)") (TriggeredSeconds :type "Float (double-precision)") (InputAction :type "InputAction Object Reference" :default "/Game/Blueprints/Inputs/Actions/IA_Move.IA_Move"))
  (bind (_returnvalue_roll _returnvalue_pitch _returnvalue_yaw) (`KismetMathLibrary.BreakRotator` (`self.GetControlRotation`)))
  ; 키보드 Move 입력
  (:`Triggered`
    (`self.AddMovementInput` (* (`KismetMathLibrary.GetForwardVector` (`KismetMathLibrary.MakeRotator` 0.0 0.0 _returnvalue_yaw)) ActionValue_Y))
    (`self.AddMovementInput` (* (`KismetMathLibrary.GetRightVector` (`self.GetControlRotation`)) ActionValue_X))))

(event `EnhancedInput|/Game/Blueprints/Inputs/Actions/IA_Look`
  (params (ActionValue :type "Vector2D Structure") (ElapsedSeconds :type "Float (double-precision)") (TriggeredSeconds :type "Float (double-precision)") (InputAction :type "InputAction Object Reference" :default "/Game/Blueprints/Inputs/Actions/IA_Look.IA_Look"))
  ; 마우스 입력을 컨트롤러 회전에 적용
  (:`Triggered`
    (`self.AddControllerYawInput` ActionValue_X)
    (`self.AddControllerPitchInput` ActionValue_Y)))

(event `EnhancedInput|/Game/Blueprints/Inputs/Actions/IA_Attack`
  (params (ActionValue :type Boolean) (ElapsedSeconds :type "Float (double-precision)") (TriggeredSeconds :type "Float (double-precision)") (InputAction :type "InputAction Object Reference" :default "/Game/Blueprints/Inputs/Actions/IA_Attack.IA_Attack"))
  ; 입력 들어오면 공격 노드 실행 및 종료
  (:`Triggered`
    (`self.Attack`)))

(event `Attack`
  ; 입력 들어오면 공격 노드 실행 및 종료
  (if (`self.HasWeapon`)
    (switch `/Game/Blueprints/Character/ECharacterState` (`self.State_BP`)
      (:`NewEnumerator0`
        (set `self.State_BP` "NewEnumerator1")
        (`self.PlayAnimMontage` "/Game/Blueprints/Character/AM_CharacterAttack.AM_CharacterAttack" 1.0 "Atttack1"))
      (:`NewEnumerator1`
        (switch `name` (`AnimInstance.Montage_GetCurrentSection` (`SkeletalMeshComponent.GetAnimInstance` (`self.Mesh`)) null)
          (:`Attack1`
            (set `self.NextCombo` "Attack2"))
          (:`Attack2`
            (set `self.NextCombo` "Attack3"))
          (:`Attack3`
            (set `self.NextCombo` "Attack4")))))))

(event `AttackEnd`
  ; 입력 들어오면 공격 노드 실행 및 종료
  (set `self.State_BP` "NewEnumerator0")
  (set `self.NextCombo` "None"))

(event `OnWeaponCollected`
  (params (WeaponActor :type "Actor Object Reference"))
  ; 무기 수집
  (`self.SetOwner` WeaponActor self)
  (`self.K2_AttachToComponent` WeaponActor (`self.Mesh`) "WeaponPosition" "SnapToTarget" "SnapToTarget" "SnapToTarget" true)
  (set `self.HasWeapon` true)
  (bind _asbp_weapon (cast `/Game/Blueprints/Character/BP_Weapon` WeaponActor))
  (set `self.Weapon` _asbp_weapon))

(event `OnAttackCheckBegin`
  ; 무기 수집
  (`/Game/Blueprints/Character/BP_Weapon.OnAttackCheckBegin` (`self.Weapon`)))

(event `OnAttackCheckEnd`
  ; 무기 수집
  (`/Game/Blueprints/Character/BP_Weapon.OnAttackCheckEnd` (`self.Weapon`)))

(fn `UserConstructionScript`)