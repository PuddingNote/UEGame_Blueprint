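; BP_MonsterBear is a bear monster actor that takes damage, shows its health on a widget bar and dies.
; AnyDamage feeds the DamageReceiver component, whose health and death events update the WBP_HP bar and trigger death.
; A timeline drives the HitValue parameter on a dynamic stone material as a hit effect.
; Death disables capsule collision, sets a final state that SetState never leaves, then destroys the actor after a delay.
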(event `self.ReceiveBeginPlay`
  (bind _returnvalue (`PrimitiveComponent.CreateDynamicMaterialInstance` (`self.Mesh`) 0 "/Game/InfinityBladeAdversaries/Enemy/Enemy_Bear/Materials/M_Bear_Stone_Inst.M_Bear_Stone_Inst" "None"))
  (set `self.DynamicInstance` _returnvalue)
  ; OnDead 이벤트에 함수 구독
  (add `/Game/Blueprints/Components/BP_DamageReceiver.OnDead` (`self.DamageReceiver`) (delegate `OnMonsterDead`))
  (bind _aswbp_hp (cast `/Game/UI/WidgetBlueprints/WBP_HP` (`WidgetComponent.GetUserWidgetObject` (`self.HPBar`))))
  (set `self.HPBarObject` _aswbp_hp)
  (add `/Game/Blueprints/Components/BP_DamageReceiver.OnHealthPowerChanged` (`self.DamageReceiver`) (delegate `OnHPChanged`)))

(event `OnHPChanged`
  (params (HealthPower :type "Float (double-precision)") (MaxHealthPower :type "Float (double-precision)"))
  (`/Game/UI/WidgetBlueprints/WBP_HP.Set HP Percent` (`self.HPBarObject`) (/ HealthPower MaxHealthPower)))

(event `OnMonsterDead`
  ; 죽으면 콜리전 끄기
  (`PrimitiveComponent.SetCollisionEnabled` (`self.CapsuleComponent`) "NoCollision")
  (`self.SetState` "NewEnumerator3")
  (`KismetSystemLibrary.Delay` 3.0)
  (`self.K2_DestroyActor`))

(event `SetState`
  (params (NewState :type "/Game/Blueprints/Monster/EMonsterState Enum" :default "NewEnumerator0"))
  (if (`|EnumInequality` (`self.State_BP`) "NewEnumerator3")
    (if (`|EnumInequality` NewState (`self.State_BP`))
      (set `self.State_BP` NewState))))

(event `self.ReceiveAnyDamage`
  (params (Damage :type "Float (single-precision)") (DamageType :type "DamageType Object Reference") (InstigatedBy :type "Controller Object Reference") (DamageCauser :type "Actor Object Reference"))
  ; 데미지 처리
  (`/Game/Blueprints/Components/BP_DamageReceiver.OnDamageReceived` (`self.DamageReceiver`) Damage)
  ; 피격 머티리얼 효과 적용
  (bind (_direction _value) (`Timeline|HitEffect` :!via `PlayFromStart`) ; Add Timeline
    (:`Update`
      (`MaterialInstanceDynamic.SetScalarParameterValue` (`self.DynamicInstance`) "HitValue" _value))))

(fn `UserConstructionScript`)