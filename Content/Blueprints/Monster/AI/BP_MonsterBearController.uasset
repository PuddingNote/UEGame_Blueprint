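; BP_MonsterBearController is the AI controller for the bear monster.
; On possession it initializes the BB_MonsterBear blackboard with the patrol wait time and the pawn's current location as its origin.
; It then runs the BT_MonsterBear behavior tree, using a Sequence node to keep blackboard setup ahead of the tree start.
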(event `self.ReceivePossess`
  (params (PossessedPawn :type "Pawn Object Reference"))
  (`|ExecutionSequence`
    (:`then_0`
      (`self.UseBlackboard` "/Game/Blueprints/Monster/AI/BB_MonsterBear.BB_MonsterBear")
      (`BlackboardComponent.SetValueAsFloat` (`self.Blackboard`) (`self.PatrolWaitTimeKey`) (`self.PatrolWaitTime`))
      (`BlackboardComponent.SetValueAsVector` (`self.Blackboard`) (`self.OriginLoactionKey`) (`self.K2_GetActorLocation` PossessedPawn)))
    (:`then_1`
      (`self.RunBehaviorTree` "/Game/Blueprints/Monster/AI/BT_MonsterBear.BT_MonsterBear"))))

(fn `UserConstructionScript`)